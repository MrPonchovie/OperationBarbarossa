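; T34 tank actor that fires blindly along its guns' facing, with no target selection, until explosive damage destroys it.
; A delayed loop from BeginPlay randomly triggers machine gun bursts or delayed main gun shots.
; Each shot spawns a projectile with cone spread, then restores aim from a reference component.
; Only radial damage above a threshold reduces health, minus a flat offset; zero health triggers Explode, setting Dead.
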(event Game|Damage|EventRadialDamage
  (params (DamageReceived :type Float%20%28single-precision%29) (DamageType :type Damage%20Type%20Object%20Reference) (Origin :type Vector :default "0, 0, 0") (HitInfo :type Hit%20Result%20Structure%20%28by%20ref%29) (InstigatedBy :type Controller%20Object%20Reference) (DamageCauser :type Actor%20Object%20Reference))
  (if (not (Variables|Default|Getdead))
    (if (< 99.0 DamageReceived)
      (bind _output_get (Variables|Default|SetHealth (- (Variables|Default|GetHealth) (- (Math|Float|Truncate DamageReceived) 50))))
      (Development|PrintString (Utilities|String|BuildString(Integer) (Utilities|String|ToString(Float) DamageReceived) "Health:" (Variables|Default|GetHealth)))
      (if (<= _output_get 0)
        (CallFunction|Explode)))))

(event EventBeginPlay
  (Variables|Default|SetBone%20Names (Transformation|GetAllSocketNames (Variables|Default|GetSkeletalMesh)))
  (Utilities|ForLoopwithDelayWW2 0 9000 1.0
    (:Body
      (if (Variables|Default|Getdead)
        (Development|PrintString "oof")
        (else
          (bind _output_get (Variables|Default|SetRandom (Math|Random|RandomIntegerinRange 1 6)))
          (if (== _output_get 1)
            (bind _output_get_2 (Variables|Default|SetBurst (Math|Random|RandomIntegerinRange 8 35)))
            (Utilities|ForLoopwithDelayWW2 0 _output_get_2 0.09
              (:Body
                (CallFunction|ShootMachineGun)))
            (elif (== _output_get 6)
              (GameplayTasks|TaskWaitDelay (Variables|Default|GetGameplayTasks) (Math|Random|RandomFloatinRange 5.0 15.0)
                (:OnFinish
                  (if (not (Variables|Default|Getdead))
                    (CallFunction|ShootMainGun)))))))))))

(fn ConstructionScript
  (for _array_element (Variables|Default|GetBone%20Names)
    _))

(fn ShootMainGun
  (bind _tankgun (Variables|Default|GetTankGun))
  (Transformation|SetWorldRotation (Variables|Default|GetTankGun) (Math|Conversions|RotationFromXVector (Math|Random|RandomUnitVectorinConeinDegrees (Math|Vector|GetForwardVector (Variables|Default|GetTankGun)) 2.0)) false true)
  (Effects|SpawnEmitterAttached "/HDCore/Effects/Particles/Backblast/P_AT4_BackBlast.P_AT4_BackBlast" (Variables|Default|GetTankGun) "None")
  (Audio|PlaySoundatLocation "/HDAssets/Audio/Weapon/SoundCues/Explosions/A_AT4_Shoot.A_AT4_Shoot" (Transformation|GetWorldLocation _tankgun) "0, 0, 0" 1.0 1.0 0.0 0 0 0)
  (Game|SpawnActorfromClass "/OperationBarbarossa/Blueprints/ZIS-3/BP_ZIS-2_Shell.BP_ZIS-2_Shell_C" (Transformation|GetSocketTransform _tankgun "None" "RTS_World") "Undefined" 0 (CallFunction|GetHDPlayerCharacterBP))
  (Transformation|SetWorldRotation (Variables|Default|GetTankGun) (Transformation|GetWorldRotation (Variables|Default|GetTankGun1)) false false))

(fn ShootMachineGun
  (bind _machinegun (Variables|Default|GetMachineGun))
  (bind _machinegun_2 (Variables|Default|GetMachineGun))
  (Transformation|SetWorldRotation _machinegun (Math|Conversions|RotationFromXVector (Math|Random|RandomUnitVectorinConeinDegrees (Math|Vector|GetForwardVector _machinegun) 2.0)) false true)
  (Effects|SpawnEmitterAttached "/HDCore/Effects/Particles/MuzzleFX/P_Muzzleflash_MG_Star.P_Muzzleflash_MG_Star" (Variables|Default|GetMachineGun) "None")
  (Audio|PlaySoundatLocation "/HDAssets/Audio/Weapon/SoundCues/MG/PKM/A_PKM_FIELD_Cue.A_PKM_FIELD_Cue" (Transformation|GetWorldLocation _machinegun_2) "0, 0, 0" 1.0 1.0 0.0 0 0 0)
  (Game|SpawnActorfromClass "/HDAssets/Items/Weapons/MachineGuns/PKM_P/BP_HDProj_PKM_P_Weap.BP_HDProj_PKM_P_Weap_C" (Transformation|GetSocketTransform _machinegun_2 "None" "RTS_World") "AlwaysSpawn" 0 (Game|GetInstigator))
  (Transformation|SetWorldRotation (Variables|Default|GetMachineGun) (Transformation|GetWorldRotation (Variables|Default|GetMachineGun1)) false false))

(fn Explode
  (bind _defaultsceneroot (Variables|Default|GetDefaultSceneRoot))
  (bind _returnvalue (Transformation|GetWorldLocation _defaultsceneroot))
  (Effects|SpawnEmitteratLocation "/HDAssets/Vehicles/HMV/PS_Vehicle_Explosion.PS_Vehicle_Explosion" _returnvalue "0, 0, 0" "3.000000,3.000000,3.000000")
  (Audio|PlaySoundatLocation "/HDAssets/Audio/Weapon/SoundCues/Explosions/A_Rocket_Explosion.A_Rocket_Explosion" _returnvalue "0, 0, 0" 1.0 1.0 0.0 0 0 0)
  (Variables|Default|Setdead true)
  (Transformation|SetWorldScale3D (Variables|Default|GetParticleSystem) "1.000000,1.000000,1.000000"))