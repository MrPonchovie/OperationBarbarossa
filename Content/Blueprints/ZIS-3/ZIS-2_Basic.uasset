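; AI-crewed ZIS-2 gun tied to a capture point, destroying itself if that point's active route differs from its own.
; While any crew lives and the enemy can capture the point, it fires on randomised timers via a server event and multicast, spawning shells with cone spread and effects.
; When another team takes the point, a fully dead crew respawns, though both new crewmen are stored in CrewMember1 without team assignment.
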(event Custom|OnOwningTeamUpdate_Event_0
  (params (ControlPoint :type HD%20Base%20Capture%20Point%20Object%20Reference) (PrevTeam :type EHDTeam%20Enum :default "Red") (NewTeam :type EHDTeam%20Enum :default "Red") (bCaptured :type Boolean))
  ;[1 1 1] Startup code, like getting respawns ready and seeing if i should exist
  (if (!= (Class|DFBlueprintFunctions|GetTeamNum (CallFunction|GetBluforOpforTeamStateforTeam NewTeam)) (Variables|Default|GetMy%20Team))
    (bind _crewisdead_ (CallFunction|CrewDeadQuery))
    (if _crewisdead_
      (CallFunction|RespawnCrew))))

(event Custom|Multicast_Shoot_Event
  ;[1 1 1] Code for shooting
  (Transformation|SetWorldRotation (Variables|Default|GetBarrelEnd) (Math|Conversions|RotationFromXVector (Math|Random|RandomUnitVectorinConeinDegrees (Math|Vector|GetForwardVector (Variables|Default|GetBarrelEnd)) 2.0)) false true)
  (Audio|Components|Audio|Play (Variables|Default|GetCameraShakeSource))
  (Effects|SpawnEmitteratLocation "/HDCore/Effects/Particles/Backblast/P_AT4_BackBlast.P_AT4_BackBlast" (Transformation|GetWorldLocation (Variables|Default|GetBarrelEnd)) (Math|Conversions|RotationFromXVector (Math|Vector|GetForwardVector (Variables|Default|GetBarrelEnd))))
  (Audio|Components|Audio|Play (Variables|Default|GetAudio) 0.0)
  (Game|SpawnActorfromClass "/OperationBarbarossa/Blueprints/ZIS-3/BP_ZIS-2_Shell.BP_ZIS-2_Shell_C" (Transformation|GetSocketTransform (Variables|Default|GetBarrelEnd) "None" "RTS_World") "AlwaysSpawn" 0 0)
  (Transformation|SetWorldRotation (Variables|Default|GetBarrelEnd) (Transformation|GetWorldRotation (Variables|Default|GetBarrelEnd1)) false false))

(event Custom|Server_Shoot_Event
  (params (Target :type ZIS-2%20Basic%20Object%20Reference))
  ;[1 1 1] Code for shooting
  (CallFunction|MulticastShootEvent))

(event EventBeginPlay
  ;[1 1 1] Startup code, like getting respawns ready and seeing if i should exist
  (bind _output_get (Variables|Default|SetCrewMember1 (Variables|/Script/Engine.ChildActorComponent|GetChildActor (Variables|Default|GetZIS-2_Crew))))
  (bind _output_get_2 (Variables|Default|SetCrewMember2 (Variables|/Script/Engine.ChildActorComponent|GetChildActor (Variables|Default|GetZIS-2_Crew1))))
  (CallFunction|SetCrewTeams (Utilities|Array|MakeArray _output_get_2 _output_get))
  (bind _asbp_hdcapture_point_base (Utilities|Casting|CastToBP_HDCapturePointBase (Variables|Default|GetBoundFlag)))
  (if (== (Variables|/Script/HDMain.HDBaseCapturePoint|GetActiveRoute _asbp_hdcapture_point_base) (Variables|Default|GetMy%20Route))
    (EventDispatchers|AssignOnOwningTeamUpdate _asbp_hdcapture_point_base (delegate Custom|OnOwningTeamUpdate_Event_0))
    ;[1 1 1] Determines if i can shoot
    (Utilities|ForLoopwithDelayWW2 0 900 1e+01
      (:Body
        (GameplayTasks|TaskWaitDelay (Variables|Default|GetGameplayTasks) (Math|Random|RandomFloatinRange 0.0 15.0)
          (:OnFinish
            (bind _crewisdead_ (CallFunction|CrewDeadQuery))
            (if (not _crewisdead_)
              (if (Class|HDBaseCapturePoint|IsCapturablebyTeam _asbp_hdcapture_point_base (Variables|Default|GetEnemy%20Team))
                (CallFunction|ServerShootEvent)))))))
    (else
      (Actor|DestroyActor))))

(fn ConstructionScript)

(fn CrewDeadQuery
  (bind _aszis_2_crew (Utilities|Casting|CastToZIS-2_Crew (Variables|Default|GetCrewMember1))
    (:then
      (if (Variables|/OperationBarbarossa/Blueprints/ZIS-3/ZIS-2_Crew.ZIS-2_Crew_C|GetDead _aszis_2_crew)
        (LocalVariables|SetAmountDead (+ (LocalVariables|GetAmountDead) 1) :!label _label)))
    (:CastFailed
      (goto _label)))
  (bind _aszis_2_crew_2 (Utilities|Casting|CastToZIS-2_Crew (Variables|Default|GetCrewMember2))
    (:then
      (if (Variables|/OperationBarbarossa/Blueprints/ZIS-3/ZIS-2_Crew.ZIS-2_Crew_C|GetDead _aszis_2_crew_2)
        (bind _output_get (LocalVariables|SetAmountDead (+ (LocalVariables|GetAmountDead) 1) :!label _label_2))))
    (:CastFailed
      (goto _label_2)))
  (if (< _output_get 2)
    (Development|PrintString "Crew Alive")
    (return false)
    (else
      (Development|PrintString "Crew Dead")
      (return true))))

(fn RespawnCrew
  (Actor|DestroyActor (Variables|Default|GetCrewMember1))
  (Actor|DestroyActor (Variables|Default|GetCrewMember2))
  (bind _returnvalue (Game|SpawnActorfromClass "/OperationBarbarossa/Blueprints/ZIS-3/ZIS-2_Crew.ZIS-2_Crew_C" (Transformation|GetWorldTransform (Variables|Default|GetCrew%20Spot%201)) "Undefined" self false 0))
  (Variables|Default|SetCrewMember1 _returnvalue)
  (bind _returnvalue_2 (Game|SpawnActorfromClass "/OperationBarbarossa/Blueprints/ZIS-3/ZIS-2_Crew.ZIS-2_Crew_C" (Transformation|GetWorldTransform (Variables|Default|GetCrew%20Spot%202)) "Undefined" self false 0))
  (Variables|Default|SetCrewMember1 _returnvalue_2)
  (Development|PrintString "Respawned Crew!"))

(fn SetCrewTeams
  (params (Crew :type Array%20of%20Actor%20Object%20References))
  (for _array_element Crew
    (bind _aszis_2_crew (Utilities|Casting|CastToZIS-2_Crew _array_element))
    (Variables|/OperationBarbarossa/Blueprints/ZIS-3/ZIS-2_Crew.ZIS-2_Crew_C|SetCrew%20Team _aszis_2_crew (Variables|Default|GetMy%20Team))))