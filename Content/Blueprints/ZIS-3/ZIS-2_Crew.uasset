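; Crew member for the ZIS-2 gun that takes damage, dies and shouts periodic voice barks.
; Point and radial damage pass the instigator's team through server and multicast events, which ignore same-team hits and subtract Health.
; At zero Health it sets Dead, plays a death sound and ragdolls the crew mesh, with debug prints.
; From BeginPlay, a delayed loop with random offsets plays suppressing barks while alive.
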(event Custom|Server_TakenDamage_Event
  (params (InFloat :type Float%20%28single-precision%29) (B :type EHDTeam%20Enum :default "Red"))
  ;[1 1 1] Taking Damage and Death
  (CallFunction|MulticastTakenDamageEvent InFloat B))

(event Custom|Multicast_TakenDamage_Event
  (params (InFloat :type Float%20%28single-precision%29) (B :type EHDTeam%20Enum :default "Red"))
  ;[1 1 1] Taking Damage and Death
  (if (not (Utilities|Enum|Equal(Enum) B (Variables|Default|GetCrew%20Team)))
    (if (not (Variables|Default|Getdead))
      (bind _output_get (Variables|Default|SetHealth (- (Variables|Default|GetHealth) (Math|Float|Truncate InFloat))))
      (Development|PrintString (Utilities|String|BuildString(Integer) (Utilities|String|ToString(Float) InFloat) "Health:" (Variables|Default|GetHealth)))
      (if (<= _output_get 0)
        (Variables|Default|SetDead true)
        (Audio|PlaySoundatLocation "/HDAssets/Characters/Common/Audio/VO/RU/A_RU_Dead.A_RU_Dead" (Transformation|GetWorldLocation (Variables|Default|GetCrew%20Mesh)) "0, 0, 0" 1.0 1.0 0.0 0 0 self)
        (Development|PrintString "I DEAD")
        (Physics|SetSimulatePhysics (Variables|Default|GetCrew%20Mesh) true)))))

(event Game|Damage|EventRadialDamage
  (params (DamageReceived :type Float%20%28single-precision%29) (DamageType :type Damage%20Type%20Object%20Reference) (Origin :type Vector :default "0, 0, 0") (HitInfo :type Hit%20Result%20Structure%20%28by%20ref%29) (InstigatedBy :type Controller%20Object%20Reference) (DamageCauser :type Actor%20Object%20Reference))
  (CallFunction|ServerTakenDamageEvent DamageReceived (Utilities|Enum|ByteToEnumEHDTeam (Class|DFBlueprintFunctions|GetTeamNum InstigatedBy))))

(event Game|Damage|EventPointDamage
  (params (Damage :type Float%20%28single-precision%29) (DamageType :type Damage%20Type%20Object%20Reference) (HitLocation :type Vector :default "0, 0, 0") (HitNormal :type Vector :default "0, 0, 0") (HitComponent :type Primitive%20Component%20Object%20Reference) (BoneName :type Name :default "None") (ShotFromDirection :type Vector :default "0, 0, 0") (InstigatedBy :type Controller%20Object%20Reference) (DamageCauser :type Actor%20Object%20Reference) (HitInfo :type Hit%20Result%20Structure%20%28by%20ref%29))
  (CallFunction|ServerTakenDamageEvent Damage (Utilities|Enum|ByteToEnumEHDTeam (Class|DFBlueprintFunctions|GetTeamNum InstigatedBy))))

(event EventBeginPlay
  ;[1 1 1] Vocal barks
  (Utilities|ForLoopwithDelayWW2 0 9999 15.0
    (:Body
      (GameplayTasks|TaskWaitDelay (Variables|Default|GetGameplayTasks) (Math|Random|RandomFloatinRange 0.0 5.0)
        (:OnFinish
          (if (not (Variables|Default|Getdead))
            (Audio|PlaySoundatLocation "/HDAssets/Characters/Common/Audio/VO/RU/A_RU_Suppressing.A_RU_Suppressing" (Transformation|GetWorldLocation (Variables|Default|GetDefaultSceneRoot)) "0, 0, 0" 1.0 1.0 0.0 0 0 0)))))))

(fn ConstructionScript)

(fn OnRepDead)