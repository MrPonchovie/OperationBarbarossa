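; Base Blueprint for USSR grenades that plays the explosion effects when the payload activates.
; Dedicated servers and projectiles with a valid predicted client counterpart skip everything, avoiding duplicate effects.
; Otherwise it plays a world camera shake, a pooled particle effect and an optional sound at its location.
; When the particle asset is valid, a runtime-added GameplayTasks component runs a short delay before firing the PhysicsBlastForce impulse.
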(event EventPayloadActivated
  (params (ImpactHitResult :type Hit%20Result%20Structure%20%28by%20ref%29))
  (if (not (or (Class|DFBaseProjectile|HasValidPredictedClientProjectile) (Networking|IsDedicatedServer))) ; Don't spawn explosion fx for this\nprojectile if a predicted one is\nassociated with it.
    (Utilities|FlowControl|Sequence
      (:then_0
        (Camera|PlayWorldCameraShake (Variables|CameraShake|GetCameraShake) (Transformation|GetActorLocation) (Variables|CameraShake|GetCameraShakeInnerRadius) (Variables|CameraShake|GetCameraShakeOuterRadius) 1.0 true)
        (bind _explosionps (Variables|Grenade|GetExplosionPS)
          (:then
            (Effects|SpawnEmitteratLocation _explosionps (Transformation|GetActorLocation) "0, 0, 0" "1.000000,1.000000,1.000000" true "AutoRelease")
            (bind _returnvalue (AddComponent|AddGameplayTasksComponent))
            (GameplayTasks|TaskWaitDelay _returnvalue 0.1
              (:OnFinish
                (Class|RadialForceComponent|FireImpulse (Variables|Default|GetPhysics%20Blast%20Force))
                (CallFunction|EndFunction))))
          (:else)))
      (:then_1
        (bind _explosionsnd (Variables|Grenade|GetExplosionSnd)
          (:then
            (Audio|PlaySoundatLocation _explosionsnd (Transformation|GetActorLocation) "0, 0, 0" 1.0 1.0 0.0 0 0 0))
          (:else))))))

(fn ConstructionScript)

(fn EndFunction)