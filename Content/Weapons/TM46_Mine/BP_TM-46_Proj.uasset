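; TM-46 mine actor that sets its instigator as owner on spawn and arms itself after a short delay.
; Once armed, DetectionBox overlaps by any player character, grenade or bullet call a multicast explode event directly.
; The explosion plays effects, sound and camera shake, fires a physics impulse, applies radial falloff damage and destroys the actor.
; A Blue-team friendly list builder exists but is never run, so triggering ignores team.
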(event OnComponentBeginOverlap(DetectionBox)
  (params (OverlappedComponent :type Primitive%20Component%20Object%20Reference) (OtherActor :type Actor%20Object%20Reference) (OtherComp :type Primitive%20Component%20Object%20Reference) (OtherBodyIndex :type Integer) (bFromSweep :type Boolean) (SweepResult :type Hit%20Result%20Structure%20%28by%20ref%29))
  (if (Variables|Default|GetArmed)
    (Utilities|Casting|CastToHDPlayerCharacter OtherActor
      (:then
        _)
      (:CastFailed
        (Utilities|Casting|CastToBP_USSR_GrenadeBase OtherActor
          (:then
            _)
          (:CastFailed
            (Utilities|Casting|CastToBP_HDProj_GrenadeBase OtherActor
              (:then
                _)
              (:CastFailed
                (Utilities|Casting|CastToHDProj_Bullet OtherActor)))))))
    (CallFunction|MulticastCallExplodeEvent)))

(event Custom|Server_CallExplode_Event
  (CallFunction|MulticastCallExplodeEvent))

(event Custom|Multicast_CallExplode_Event
  (bind _defaultsceneroot (Variables|Default|GetDefaultSceneRoot))
  (bind _returnvalue (Transformation|GetWorldLocation _defaultsceneroot))
  (Development|PrintString "boom")
  (Effects|SpawnEmitteratLocation "/HDCore/Effects/Particles/Explosions/PS_Rocket_Explosion_Dust.PS_Rocket_Explosion_Dust" _returnvalue "0, 0, 0" "1.000000,1.000000,1.000000" true "AutoRelease")
  (Audio|PlaySoundatLocation "/HDAssets/Items/Common/Audio/A_Grenade_Explosion_Cue.A_Grenade_Explosion_Cue" _returnvalue "0, 0, 0" 1.0 1.0 0.0 0 0 0)
  (Audio|Components|Audio|Play (Variables|Default|GetCameraShakeSource))
  (Class|RadialForceComponent|FireImpulse (Variables|Default|GetPhysics%20Blast%20Force))
  (Class|GameplayStatics|ApplyRadialDamagewithFalloff 2e+02 5e+01 (+ (Transformation|GetWorldLocation (Variables|Default|GetDefaultSceneRoot)) "0, 0,5.000000") 5e+01 7e+02 0.3 "/Script/Engine.DamageType" 0 self (Game|GetInstigatorController) "ECC_WorldStatic")
  (Actor|DestroyActor))

(event Custom|NewEventDispatcher_0_Event)

(event EventBeginPlay
  (bind _instigator (Variables|Actor|GetInstigator))
  (Development|PrintString (Utilities|String|Append "Began play with owner being: " (Utilities|GetObjectName _instigator)))
  (Actor|SetOwner _instigator)
  (GameplayTasks|TaskWaitDelay (Variables|Default|GetGameplayTasks) 5.0
    (:OnFinish
      (Variables|Default|SetArmed true))))

(event Game|Damage|EventPointDamage
  (params (Damage :type Float%20%28single-precision%29) (DamageType :type Damage%20Type%20Object%20Reference) (HitLocation :type Vector :default "0, 0, 0") (HitNormal :type Vector :default "0, 0, 0") (HitComponent :type Primitive%20Component%20Object%20Reference) (BoneName :type Name :default "None") (ShotFromDirection :type Vector :default "0, 0, 0") (InstigatedBy :type Controller%20Object%20Reference) (DamageCauser :type Actor%20Object%20Reference) (HitInfo :type Hit%20Result%20Structure%20%28by%20ref%29)))

(fn ConstructionScript)

(fn SetFriendlyTeam
  (bind _hdteamstate (CallFunction|GetHDTeamStateforTeam "Blue"))
  (bind _returnvalue (Class|HDTeamState|GetPlatoonat _hdteamstate 0 false))
  (bind _output_get (Variables|Default|SetNumber%20of%20Blue%20Squads (Class|HDPlatoonState|GetNumSquads _returnvalue false)))
  (for _index (range 0 _output_get)
    (for _index_2 (range 0 (Class|HDSquadState|GetNumSquadMembers (Class|HDPlatoonState|GetSquadat _returnvalue _index false) false))
      (Development|PrintString (PlayerState|GetPlayerName (Class|HDSquadState|GetSquadMemberat (Class|HDPlatoonState|GetSquadat _returnvalue _index false) _index_2 false)))
      (Utilities|Array|AppendArray (Variables|Default|GetFriendly%20Team) (Utilities|Array|MakeArray (Variables|/Script/Engine.PlayerState|GetPawnPrivate (Class|HDSquadState|GetSquadMemberat (Class|HDPlatoonState|GetSquadat _returnvalue _index false) _index_2 false))))))
  (return (Variables|Default|GetFriendly%20Team)))